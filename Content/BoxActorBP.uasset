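; BoxActorBP is a labelled box actor whose static mesh resizes to fit its text.
; FitText, run from the construction script and the SizeFitContents event, scales the mesh from the text's local size plus a margin and a set depth, then offsets the text within it.
; An unconnected box-repulsion graph, which never runs, would add velocity pushing the box away from other BoxActorBP instances within RepulsionDistance.
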(event `self.SizeFitContents`
  (`self.FitText`))

(fn `FitText`
  (bind _labelmargin (`self.LabelMargin`))
  (bind _returnvalue (* (`self.LabelMargin`) 2.0))
  (bind _returnvalue_2 (+ _returnvalue (.y (`TextRenderComponent.GetTextLocalSize` (`self.TextRender`)))))
  (bind _returnvalue_3 (+ (.z (`TextRenderComponent.GetTextLocalSize` (`self.TextRender`))) _returnvalue))
  (`SceneComponent.SetRelativeScale3D` (`self.StaticMesh`) (/ (`KismetMathLibrary.MakeVector` _returnvalue_2 (`self.Depth`) _returnvalue_3) 100.0))
  (`SceneComponent.K2_SetRelativeLocation` (`self.TextRender`) (`KismetMathLibrary.MakeVector` (+ (/ _returnvalue_2 -2.0) _labelmargin) 0.0 (+ _labelmargin (/ _returnvalue_3 -2.0))) false false))

(fn `UserConstructionScript`
  (set `self.mainLabel` (`self.TextRender`))
  (set `self.cube` (`self.StaticMesh`))
  (`self.FitText`))