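; BP_Mat_with_Slider is a display actor that lets a slider drive a material's "Value" parameter on a preview mesh.
; The construction script optionally swaps in a scaled sphere mesh, creates the dynamic material instance and initializes the parameter and labels.
; While the capsule overlap flags PlayerNear, Tick maps the slider between min and max into that parameter.
; HasVariable toggles showing the variable's name and live value.
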(event `self.ReceiveTick`
  (params (DeltaSeconds :type "Float (single-precision)"))
  (bind _valuetext (`self.ValueText`))
  (bind _returnvalue (`KismetMathLibrary.Lerp` (`self.SliderMin`) (`self.Slider Max`) (`/Game/ExampleContent/AnimationDemo/BluePrints/BP_Slider.Value` (`self.Slider`))))
  (if (`self.PlayerNear`)
    (`MaterialInstanceDynamic.SetScalarParameterValue` (`self.MID`) "Value" _returnvalue)
    (if (`self.HasVariable`)
      (`TextRenderComponent.K2_SetText` _valuetext (`KismetTextLibrary.Conv_StringToText` (`KismetStringLibrary.Conv_DoubleToString` _returnvalue)))
      (else
        (`TextRenderComponent.K2_SetText` _valuetext (`self.NewVar_0`))))))

(event `self.Capsule1.OnComponentBeginOverlap`
  (params (OtherActor :type "Actor Object Reference") (OtherComp :type "PrimitiveComponent Object Reference") (OtherBodyIndex :type Integer) (bFromSweep :type Boolean) (SweepResult :type "HitResult Structure (by ref)"))
  (set `self.PlayerNear` true))

(event `self.Capsule1.OnComponentEndOverlap`
  (params (OtherActor :type "Actor Object Reference") (OtherComp :type "PrimitiveComponent Object Reference") (OtherBodyIndex :type Integer))
  (set `self.PlayerNear` false))

(fn `UserConstructionScript`
  (bind _displaymesh (`self.Displaymesh`))
  (bind _valueheader (`self.ValueHeader`))
  (if (`self.UseSphereMesh`)
    (`|ExecutionSequence`
      (:`then_0`
        (`StaticMeshComponent.SetStaticMesh` _displaymesh "/Engine/EditorMeshes/EditorSphere.EditorSphere")
        (`SceneComponent.SetWorldScale3D` _displaymesh (`KismetMathLibrary.Conv_DoubleToVector` (`self.SphereSize`)))
        (`SceneComponent.K2_SetRelativeLocation` _displaymesh (`KismetMathLibrary.MakeVector` 0.0 0.0 (`self.SphereZLocation`)) false false))
      (:`then_1`
        (bind _returnvalue (`PrimitiveComponent.CreateDynamicMaterialInstance` (`self.Displaymesh`) 0 (`self.Material`) :!label _label))
        (set `self.MID` _returnvalue)
        (`MaterialInstanceDynamic.SetScalarParameterValue` (`self.MID`) "Value" (`self.DefaultValue`))
        (if (`self.HasVariable`)
          ;[1 1 1] Variable Text
          (`TextRenderComponent.K2_SetText` _valueheader (`self.Name of variable`))
          (`TextRenderComponent.K2_SetText` (`self.ValueText`) (`KismetTextLibrary.Conv_StringToText` (`KismetStringLibrary.Conv_DoubleToString` (`self.DefaultValue`))))
          (else
            (`TextRenderComponent.K2_SetText` _valueheader (`self.NewVar_0`))
            (`TextRenderComponent.K2_SetText` (`self.ValueText`) (`self.NewVar_0`))))))
    (else
      (goto _label))))