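; FrameBP is a frame actor that groups nested box actors and spaces them apart with physics each tick.
; It computes the boxes' bounds, moves Min and Max markers there, and stores the unhalved corner sum as CenterNested.
; Nearby boxes repel each other through added velocity, and a global FrameBP search pushes close frames' contents apart along X.
; An alternative linked NextFrame spacing graph is never executed.
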(event `self.ReceiveTick`
  (params (DeltaSeconds :type "Float (single-precision)"))
  (bind _minnested (`self.MinNested`))
  (bind _maxnested (`self.MaxNested`))
  ;[1 1 1] Bounds Determination
  (bind (_box _index) (`self.ForEachNestedBoxActor` self)
    (:`Body`
      (if (== 0 _index)
        (bind _returnvalue (`self.K2_GetActorLocation` _box))
        (set `self.MaxNested` _returnvalue)
        (set `self.MinNested` _returnvalue)
        (else
          (bind _x (.x _returnvalue))
          (bind _y (.y _returnvalue))
          (bind _z (.z _returnvalue))
          (set `self.MinNested` (`KismetMathLibrary.MakeVector` (`KismetMathLibrary.FMin` (.x (`self.MinNested`)) _x) (`KismetMathLibrary.FMin` (.y (`self.MinNested`)) _y) (`KismetMathLibrary.FMin` (.z (`self.MinNested`)) _z)))
          (set `self.MaxNested` (`KismetMathLibrary.MakeVector` (`KismetMathLibrary.FMax` _x (.x (`self.MaxNested`))) (`KismetMathLibrary.FMax` _y (.y (`self.MaxNested`))) (`KismetMathLibrary.FMax` _z (.z (`self.MaxNested`))))))))
    (:`Done`
      (`SceneComponent.K2_SetWorldLocation` (`self.Min`) _minnested false false)
      (`SceneComponent.K2_SetWorldLocation` (`self.Max`) _maxnested false false)
      (set `self.CenterNested` (+ _minnested _maxnested))
      ;[1 1 1] Box Repulsion
      (bind _box_2 (`self.ForEachNestedBoxActor` null)
        (:`Body`
          (bind _box_3 (`self.ForEachNestedBoxActor` null)
            (:`Body`
              (if (and (>= 200.0 (`self.GetDistanceTo` _box_2 _box_3)) (!= _box_2 _box_3))
                (`PrimitiveComponent.SetPhysicsLinearVelocity` (`/Game/Blueprints/BoxActorBP.Box` _box_2) (* (`KismetMathLibrary.GetForwardVector` (`KismetMathLibrary.FindLookAtRotation` (`SceneComponent.K2_GetComponentLocation` (`self.K2_GetRootComponent` _box_3)) (`SceneComponent.K2_GetComponentLocation` (`self.K2_GetRootComponent` _box_2)))) 9.0) true "None")))
            (:`Done`
              ;[1 1 1] Frame Repulsion
              (bind _outactors (`GameplayStatics.GetAllActorsOfClass` "FrameBP_C"))
              (for _array_element _outactors
                (bind _asframe_bp (cast `/Game/Blueprints/FrameBP` _array_element))
                (bind _centernested (`/Game/Blueprints/FrameBP.CenterNested` _asframe_bp))
                (if (and (!= self _array_element) (>= 500.0 (`KismetMathLibrary.VSize` (- _centernested (`self.CenterNested`)))))
                  (for _array_element_2 (`self.Nested`)
                    (bind _asbox_collision (cast `BoxComponent` (`self.K2_GetRootComponent` _array_element_2)))
                    (`PrimitiveComponent.SetPhysicsLinearVelocity` _asbox_collision (* (`KismetMathLibrary.MakeVector` (.x (`KismetMathLibrary.GetForwardVector` (`KismetMathLibrary.FindLookAtRotation` _centernested (`self.CenterNested`))))) 3.0) true "None")))))))))))

(fn `UserConstructionScript`)