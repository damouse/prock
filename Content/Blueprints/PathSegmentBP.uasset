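; PathSegmentBP draws a path segment as parallel spline meshes linking two BoxActorBP actors, Start and End.
; Construction rebuilds the spline mesh components under Box, then Redraw positions them, as it also does on BeginPlay and NeedsRedraw.
; Redraw picks either path point on each actor via connect flags, derives tangents through CalculateEntryTangent, and offsets each spline along a fixed Y axis in Box space.
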(event `self.ReceiveTick`
  (params (DeltaSeconds :type "Float (single-precision)")))

(event `self.ReceiveBeginPlay`
  (`self.Redraw` :!label _label))

(event `self.NeedsRedraw`
  (goto _label))

(fn `Initialize`
  (`KismetArrayLibrary.Array_Clear` (`self.Splines`))
  (for _ (range 6)
    (bind _returnvalue (`AddComponent|NODE_AddSplineMeshComponent-0`))
    (`SceneComponent.K2_AttachToComponent` _returnvalue (`self.Box`) "None" "KeepWorld" "SnapToTarget" "SnapToTarget" false)
    (`KismetArrayLibrary.Array_Add` (`self.Splines`) _returnvalue)))

(fn `IsAttachmentParent`
  (params (AttachObject :type "BoxActor Object Reference"))
  (returns (ReturnValue :type Boolean))
  (return (== (`self.K2_GetRootComponent` AttachObject) (`SceneComponent.GetAttachParent` (`self.Box`)))))

(fn `PrintExtent`
  (params (Origin :type "Vector Structure") (Extent :type "Vector Structure"))
  (`KismetSystemLibrary.PrintString` (`KismetStringLibrary.Conv_VectorToString` Origin) true true (struct :`R` 0.284048 :`G` 0.900174 :`B` 1.0 :`A` 1.0) 100.0)
  (`KismetSystemLibrary.PrintString` (`KismetStringLibrary.Conv_VectorToString` Extent) true true (struct :`R` 1.0 :`G` 0.788013 :`B` 0.491394 :`A` 1.0) 100.0))

(fn `Redraw`
  (bind _returnvalue (`SceneComponent.K2_GetComponentToWorld` (`self.Box`)))
  (bind _asbox_actor_bp (cast `/Game/Blueprints/BoxActorBP` (`self.Start`)))
  (bind (_startlocation _starttangent _endlocation) (`/Game/Blueprints/BoxActorBP.GetPathPoints` _asbox_actor_bp))
  (if (`self.ConnectToStartSource`)
    (set `self.StartPosition` _startlocation)
    (set `self.StartTangent` (`self.CalculateEntryTangent` (- _endlocation _startlocation)))
    (set `self.StartRight` (0.0 1.0 0.0))
    (else
      (set `self.StartPosition` _endlocation)
      (set `self.StartTangent` (`self.CalculateEntryTangent` (- _endlocation _startlocation)))
      (set `self.StartRight` (0.0 1.0 0.0))))
  (bind _asbox_actor_bp_2 (cast `/Game/Blueprints/BoxActorBP` (`self.End`)))
  (bind (_startlocation_2 _starttangent_2 _endlocation_2) (`/Game/Blueprints/BoxActorBP.GetPathPoints` _asbox_actor_bp_2))
  (if (`self.ConnectToEndSource`)
    (set `self.EndPosition` _startlocation_2)
    (set `self.EndTangent` (`self.CalculateEntryTangent` (- _endlocation_2 _startlocation_2)))
    (set `self.EndRight` (0.0 1.0 0.0))
    (else
      (set `self.EndPosition` _endlocation_2)
      (set `self.EndTangent` (`self.CalculateEntryTangent` (- _endlocation_2 _startlocation_2)))
      (set `self.EndRight` (0.0 1.0 0.0))))
  (for (_array_element _array_index) (`self.Splines`)
    (bind _returnvalue_2 (`KismetMathLibrary.Conv_IntToDouble` (* _array_index 2)))
    (`SplineMeshComponent.SetStartAndEnd` _array_element (`KismetMathLibrary.InverseTransformLocation` _returnvalue (+ (`self.StartPosition`) (* (`self.StartRight`) _returnvalue_2))) (`self.StartTangent`) (`KismetMathLibrary.InverseTransformLocation` _returnvalue (+ (* (`self.EndRight`) _returnvalue_2) (`self.EndPosition`))) (`self.EndTangent`) true)))

(fn `UserConstructionScript`
  (`self.Initialize`)
  (`self.Redraw`))