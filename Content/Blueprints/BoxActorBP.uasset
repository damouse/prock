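; BoxActorBP is a work-in-progress labeled box actor, with a text render and mesh, meant to nest and link to other boxes.
; It supplies socket-based line endpoints and a helper adding a spline mesh segment.
; Label fitting is stubbed, and the recursive extent printed on BeginPlay is unfinished.
; Box repulsion, splines through attached boxes and label-driven resizing exist only as disconnected graph logic.
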(event `self.ReceiveBeginPlay`
  (bind (_origin_ _newparam) (`self.GetRecursiveExtent`))
  (`KismetSystemLibrary.PrintString` "" true true (struct :`G` 1.0 :`B` 0.927246 :`A` 1.0) 71.0)
  (`KismetSystemLibrary.PrintString` (`KismetStringLibrary.Conv_VectorToString` _origin_) true true (struct :`R` 1.0 :`G` 0.054605 :`B` 0.348222 :`A` 1.0) 71.0)
  (`KismetSystemLibrary.PrintString` (`KismetStringLibrary.Conv_VectorToString` _newparam) true true (struct :`G` 0.66 :`B` 1.0 :`A` 1.0) 71.0))

(event `SetNextLine`
  (params (next :type "BoxActor Object Reference")))

(event `self.SizeFitContents`
  (`self.FitText`))

(fn `AddPathLine`
  (bind _returnvalue (`AddComponent|Spline Mesh Component_0`))
  (`SceneComponent.K2_AttachToComponent` _returnvalue (`self.Box`) "None" "KeepRelative" "KeepRelative" "KeepRelative" true)
  (`SplineMeshComponent.SetStartAndEnd` _returnvalue (-10.0 0.0 10.0) (0.0 0.0 0.0) (10.0 0.0 10.0) (0.0 0.0 0.0) true))

(fn `FitText`)

(fn `GetLineFromAttachment`
  (params (to :type "Linkable Object Reference"))
  (returns (pos :type "Vector Structure") (tan :type "Vector Structure"))
  (return (`SceneComponent.GetSocketLocation` (`self.StaticMesh`) "SocketRight") (20.0 0.0 0.0)))

(fn `GetLineToAttachment`
  (params (from :type "Linkable Object Reference"))
  (returns (pos :type "Vector Structure") (tan :type "Vector Structure"))
  (return (`SceneComponent.GetSocketLocation` (`self.StaticMesh`) "SocketLeft") (20.0 0.0 0.0)))

(fn `GetRecursiveExtent`
  (returns (`Origin ` :type "Vector Structure") (NewParam :type "Vector Structure"))
  (if (!= 0 (`KismetArrayLibrary.Array_Length` (`self.GetAttachedActors`)))
    (for _array_element (`self.GetAttachedActors`)
      (bind _asbox_actor_bp (cast `/Game/Blueprints/BoxActorBP` _array_element)))))

(fn `UserConstructionScript`
  (set `self.mainLabel` (`self.TextRender`))
  (set `self.cube` (`self.StaticMesh`))
  (`self.FitText`))