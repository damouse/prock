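; Ghost actor that wraps a BoxActorBP child actor and supplies attachment points for lines along its spline mesh.
; The construction script caches the child actor as BoxInstance.
; Both attachment getters take the other actor's matching attachment position and project it onto the straight segment between the spline mesh's world-space endpoints.
; They shift that point in X by differing, opposite-signed multiples of PathOffset and return fixed, opposite vertical tangents.
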(fn `GetLineFromAttachment`
  (params (to :type "Linkable Object Reference"))
  (returns (pos :type "Vector Structure") (tan :type "Vector Structure"))
  (bind _splinemesh (`self.SplineMesh`))
  (bind _returnvalue (`SceneComponent.K2_GetComponentToWorld` _splinemesh))
  (bind _pos (`self.GetLineFromAttachment` to null))
  (return (`KismetMathLibrary.MakeVector` (+ (* (`self.PathOffset`) -2.0) (.x (`KismetMathLibrary.FindClosestPointOnSegment` _pos (`KismetMathLibrary.TransformLocation` _returnvalue (`SplineMeshComponent.GetStartPosition` _splinemesh)) (`KismetMathLibrary.TransformLocation` _returnvalue (`SplineMeshComponent.GetEndPosition` _splinemesh))))) (.y (`KismetMathLibrary.FindClosestPointOnSegment` _pos (`KismetMathLibrary.TransformLocation` _returnvalue (`SplineMeshComponent.GetStartPosition` _splinemesh)) (`KismetMathLibrary.TransformLocation` _returnvalue (`SplineMeshComponent.GetEndPosition` _splinemesh)))) (.z (`KismetMathLibrary.FindClosestPointOnSegment` _pos (`KismetMathLibrary.TransformLocation` _returnvalue (`SplineMeshComponent.GetStartPosition` _splinemesh)) (`KismetMathLibrary.TransformLocation` _returnvalue (`SplineMeshComponent.GetEndPosition` _splinemesh))))) (0.0 0.0 10.0)))

(fn `GetLineToAttachment`
  (params (from :type "Linkable Object Reference"))
  (returns (pos :type "Vector Structure") (tan :type "Vector Structure"))
  (bind _splinemesh (`self.SplineMesh`))
  (bind _returnvalue (`SceneComponent.K2_GetComponentToWorld` _splinemesh))
  (bind _pos (`self.GetLineToAttachment` from null))
  (return (`KismetMathLibrary.MakeVector` (+ (`self.PathOffset`) (.x (`KismetMathLibrary.FindClosestPointOnSegment` _pos (`KismetMathLibrary.TransformLocation` _returnvalue (`SplineMeshComponent.GetStartPosition` _splinemesh)) (`KismetMathLibrary.TransformLocation` _returnvalue (`SplineMeshComponent.GetEndPosition` _splinemesh))))) (.y (`KismetMathLibrary.FindClosestPointOnSegment` _pos (`KismetMathLibrary.TransformLocation` _returnvalue (`SplineMeshComponent.GetStartPosition` _splinemesh)) (`KismetMathLibrary.TransformLocation` _returnvalue (`SplineMeshComponent.GetEndPosition` _splinemesh)))) (.z (`KismetMathLibrary.FindClosestPointOnSegment` _pos (`KismetMathLibrary.TransformLocation` _returnvalue (`SplineMeshComponent.GetStartPosition` _splinemesh)) (`KismetMathLibrary.TransformLocation` _returnvalue (`SplineMeshComponent.GetEndPosition` _splinemesh))))) (0.0 0.0 -10.0)))

(fn `UserConstructionScript`
  (bind _asbox_actor_bp (cast `/Game/Blueprints/BoxActorBP` (`ChildActorComponent.ChildActor` (`self.Instance`))))
  (set `self.boxInstance` _asbox_actor_bp))