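; LineActorBP is a VR connection line that draws a spline mesh between two endpoints, typically boxes, and pulls those boxes together.
; Pickup stores the grabbing controller as the moving From end, and Drop reattaches the moving end to a nearby BoxActorBP.
; Tick redraws the spline from attachment points or controller position, adding opposing velocities to the boxes when their separation reaches PathOffset.
; Older ghost-connection logic remains unconnected.
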(event `/Game/Blueprints/PickupActorInterface.Drop`
  (bind _controllermovingfrom (`self.ControllerMovingFrom`))
  ;[1 1 1] Drop Event
  (if (!= _controllermovingfrom null)
    (bind _asbp_motion_controller (cast `/Game/VirtualRealityBP/Blueprints/BP_MotionController` (`ActorComponent.GetOwner` _controllermovingfrom)))
    (bind _nearestmesh (`/Game/VirtualRealityBP/Blueprints/BP_MotionController.GetActorNearHand` _asbp_motion_controller "/Game/Blueprints/BoxActorBP.BoxActorBP_C"))
    (bind _asbox_actor_bp (cast `/Game/Blueprints/BoxActorBP` _nearestmesh)
      (:`then`
        (if (!= (`self.To`) _asbox_actor_bp)
          (set `self.From` _asbox_actor_bp)))
      (:`CastFailed`
        _))
    (else
      (bind _asbp_motion_controller_2 (cast `/Game/VirtualRealityBP/Blueprints/BP_MotionController` (`ActorComponent.GetOwner` (`self.ControllerMovingTo`))))
      (bind _nearestmesh_2 (`/Game/VirtualRealityBP/Blueprints/BP_MotionController.GetActorNearHand` _asbp_motion_controller_2 "/Game/Blueprints/BoxActorBP.BoxActorBP_C"))
      (bind _asbox_actor_bp_2 (cast `/Game/Blueprints/BoxActorBP` _nearestmesh_2)
        (:`then`
          (if (!= _asbox_actor_bp_2 (`self.From`))
            (set `self.To` _asbox_actor_bp_2)))
        (:`CastFailed`
          _))))
  (set `self.ControllerMovingFrom` null)
  (set `self.ControllerMovingTo` null))

(event `/Game/Blueprints/PickupActorInterface.Pickup`
  (params (AttachTo :type "SceneComponent Object Reference"))
  (bind _returnvalue (`SceneComponent.K2_GetComponentLocation` AttachTo))
  ;[1 1 1] Pickup Event
  (if (< (`KismetMathLibrary.VSize` (- (`self.ToPos`) _returnvalue)) (`KismetMathLibrary.VSize` (- _returnvalue (`self.FromPos`))))
    (set `self.ControllerMovingFrom` AttachTo)
    (else
      (set `self.ControllerMovingFrom` AttachTo))))

(event `self.ReceiveTick`
  (params (DeltaSeconds :type "Float (single-precision)"))
  (bind _controllermovingfrom (`self.ControllerMovingFrom`))
  (bind _controllermovingto (`self.ControllerMovingTo`))
  (bind _returnvalue (* (`KismetMathLibrary.GetForwardVector` (`KismetMathLibrary.FindLookAtRotation` (`SceneComponent.K2_GetComponentLocation` (`self.K2_GetRootComponent` (`self.From`))) (`SceneComponent.K2_GetComponentLocation` (`self.K2_GetRootComponent` (`self.To`))))) (`self.AttractionVelocity`)))
  ;[1 1 1] Tick Redrawing
  (bind _bothassigned (`self.EndpointsAssigned`))
  (if _bothassigned
    (if (!= _controllermovingfrom null)
      (set `self.FromPos` (`SceneComponent.K2_GetComponentLocation` _controllermovingfrom))
      (set `self.FromTan` (0.0 0.0 0.0))
      (else
        (bind (_pos _tan) (`Linkable.GetLineFromAttachment` (`self.From`) (`self.To`)))
        (set `self.FromPos` _pos)
        (set `self.FromTan` _tan)))
    (if (!= _controllermovingto null)
      (set `self.FromPos` (`SceneComponent.K2_GetComponentLocation` _controllermovingto))
      (set `self.FromTan` (0.0 0.0 0.0))
      (else
        (bind (_pos_2 _tan_2) (`Linkable.GetLineToAttachment` (`self.To`) (`self.From`)))
        (set `self.ToPos` _pos_2)
        (set `self.ToTan` _tan_2)))
    (`SplineMeshComponent.SetStartAndEnd` (`self.SplineMesh`) (`self.FromPos`) (`self.FromTan`) (`self.ToPos`) (`self.ToTan`) true)
    ;[1 1 1] Box Attraction
    (bind (_bothassigned_2 _bothboxes) (`self.EndpointsAssigned`))
    (if _bothboxes
      (if (>= (`self.GetDistanceTo` (`self.From`) (`self.To`)) (`self.PathOffset`))
        (bind _asbox_actor_bp (cast `/Game/Blueprints/BoxActorBP` (`self.From`)))
        (bind _asbox_actor_bp_2 (cast `/Game/Blueprints/BoxActorBP` (`self.To`)))
        (`PrimitiveComponent.SetPhysicsLinearVelocity` (`/Game/Blueprints/BoxActorBP.Box` _asbox_actor_bp) _returnvalue true "None")
        (`PrimitiveComponent.SetPhysicsLinearVelocity` (`/Game/Blueprints/BoxActorBP.Box` _asbox_actor_bp_2) (`KismetMathLibrary.NegateVector` _returnvalue) true "None")))))

(fn `EndpointsAssigned`
  (returns (BothAssigned :type Boolean) (BothBoxes :type Boolean) (BothPickups :type Boolean))
  (bind _returnvalue (!= (`self.From`) null))
  (bind _returnvalue_2 (!= (`self.To`) null))
  (bind _returnvalue_3 (!= (`self.ControllerMovingFrom`) null))
  (bind _returnvalue_4 (!= (`self.ControllerMovingTo`) null))
  (return (and (or _returnvalue_3 _returnvalue) (or _returnvalue_2 _returnvalue_4)) (and _returnvalue _returnvalue_2) (and _returnvalue_3 _returnvalue_4)))

(fn `UpdateConnections`)

(fn `UserConstructionScript`)