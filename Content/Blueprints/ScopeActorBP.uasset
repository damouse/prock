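; Scope actor that tracks boxes and ghost actors, drawing parallel spline-mesh lines beneath the boxes, one per ghost.
; SetNextLine adds two spline points under each box's recursive bounds, then adds one segment per ghost, offset sideways by ghost index.
; AddNewGhost only stores and positions the ghost, without drawing lines for existing segments.
; RedrawGhosts is an empty stub, and the full-redraw loop is disconnected.
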(event `self.AddNewGhost`
  (params (ghost :type "GhostActor Object Reference") (pos :type "Vector Structure"))
  (`KismetArrayLibrary.Array_Add` (`self.Ghosts`) ghost)
  (`self.K2_SetActorLocation` ghost pos false false))

(event `self.SetNextLine`
  (params (next :type "BoxActor Object Reference"))
  (bind _returnvalue (`KismetMathLibrary.MakeVector` 0.0 0.0 1.0))
  (bind _spline (`self.Spline`))
  (bind _spline_2 (`self.Spline`))
  (bind _spline_3 (`self.Spline`))
  (bind _returnvalue_2 (`SplineComponent.GetNumberOfSplinePoints` (`self.Spline`)))
  (bind _returnvalue_3 (- _returnvalue_2 2))
  (bind _returnvalue_4 (- (`SplineComponent.GetNumberOfSplinePoints` _spline) 1))
  (bind _returnvalue_5 (- _returnvalue_2 3))
  (bind (_location _tangent) (`SplineComponent.GetLocationAndTangentAtSplinePoint` _spline_3 _returnvalue_3 "Local"))
  (bind (_location_2 _tangent_2) (`SplineComponent.GetLocationAndTangentAtSplinePoint` _spline_2 _returnvalue_5 "Local"))
  (bind _asbox_actor_bp (cast `/Game/Blueprints/BoxActorBP` next))
  (`KismetArrayLibrary.Array_Add` (`self.BoxList`) _asbox_actor_bp)
  (bind _nested (`/Game/Blueprints/BoxActorBP.GetRecursiveExtent` _asbox_actor_bp))
  (bind (_center _boxextent) (`GameplayStatics.GetActorArrayBounds` _nested))
  (bind _x (.x _center))
  (bind _y (.y _center))
  (bind _x_2 (.x _boxextent))
  (bind _returnvalue_6 (- (- (.z _center) (.z _boxextent)) 15.0))
  (`SplineComponent.AddSplinePoint` _spline (`KismetMathLibrary.MakeVector` (- _x _x_2) _y _returnvalue_6) "World" true)
  (`SplineComponent.SetTangentAtSplinePoint` _spline _returnvalue_4 _returnvalue "World" true)
  (`SplineComponent.AddSplinePoint` _spline (`KismetMathLibrary.MakeVector` (+ _x _x_2) _y _returnvalue_6) "World" true)
  (`SplineComponent.SetTangentAtSplinePoint` _spline _returnvalue_4 _returnvalue "World" true)
  (if (== (`KismetArrayLibrary.Array_Length` (`self.BoxList`)) 1)
    (`SplineComponent.SetLocationAtSplinePoint` (`self.Spline`) 0 (+ (`SplineComponent.GetLocationAtSplinePoint` (`self.Spline`) 1 "Local") (-15.0 0.0 0.0)) "Local" true))
  (for (_ _array_index) (`self.Ghosts`)
    (bind _returnvalue_7 (`AddComponent|SplineMeshComponent_0`))
    (bind _returnvalue_8 (`KismetMathLibrary.Conv_IntToDouble` (* _array_index 3)))
    (`SplineMeshComponent.SetStartAndEnd` _returnvalue_7 (+ _location_2 (* (`SplineComponent.GetRightVectorAtSplinePoint` _spline_2 _returnvalue_5 "Local") _returnvalue_8)) _tangent_2 (+ (* (`SplineComponent.GetRightVectorAtSplinePoint` _spline_3 _returnvalue_3 "Local") _returnvalue_8) _location) _tangent true)))

(event `self.RedrawGhosts`)

(fn `UserConstructionScript`)