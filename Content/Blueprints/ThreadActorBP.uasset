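; ThreadActorBP is an actor that creates a spline mesh thread between a referenced thread and a box at runtime.
; On BeginPlay it adds a manually attached spline mesh component, running from VarThreadA's spline start, converted to world space, to BoxA's location.
; An unconnected alternative spawns a SplineMeshActor with a shiny pipe mesh, attaches it to the root and sets similar endpoints without that conversion.
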(event `self.ReceiveBeginPlay`
  (bind _splinemeshcomponent (`SplineMeshActor.SplineMeshComponent` (`self.VarThreadA`)))
  (bind _returnvalue (`AddComponent|Spline Mesh Component_0` :`bManualAttachment` true))
  (`SplineMeshComponent.SetStartAndEnd` _returnvalue (`KismetMathLibrary.TransformLocation` (`SceneComponent.K2_GetComponentToWorld` _splinemeshcomponent) (`SplineMeshComponent.GetStartPosition` _splinemeshcomponent)) (0.0 0.0 0.0) (`self.K2_GetActorLocation` (`self.BoxA`)) (0.0 0.0 0.0) true))

(fn `UserConstructionScript`)