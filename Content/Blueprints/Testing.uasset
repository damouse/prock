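; Test Blueprint that generates a set of parallel copies of its Spline component in the Construction Script.
; Each pass adds a spline component, clears its default points, then rebuilds it from the source points, shifted along their local right vectors by an offset that grows with the loop index.
; Point types are copied, and each source tangent sets both arrive and leave tangents.
; The Event Graph has no active logic.
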(fn `UserConstructionScript`
  (bind _spline (`self.Spline`))
  (for _index (range 11)
    (bind _returnvalue (`AddComponent|Spline Component_0`))
    (`SplineComponent.RemoveSplinePoint` _returnvalue 0 true)
    (`SplineComponent.RemoveSplinePoint` _returnvalue 0 true)
    (for _index_2 (range (`SplineComponent.GetNumberOfSplinePoints` (`self.Spline`)))
      (bind (_location _tangent) (`SplineComponent.GetLocationAndTangentAtSplinePoint` _spline _index_2 "Local"))
      (`SplineComponent.AddSplinePoint` _returnvalue (+ (* (`SplineComponent.GetRightVectorAtSplinePoint` _spline _index_2 "Local") (`KismetMathLibrary.Conv_IntToDouble` (* _index 3))) _location) "Local" true)
      (`SplineComponent.SetSplinePointType` _returnvalue _index_2 (`SplineComponent.GetSplinePointType` _spline _index_2) true)
      (`SplineComponent.SetTangentsAtSplinePoint` _returnvalue _index_2 _tangent _tangent "Local" true))))