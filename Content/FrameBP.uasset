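; FrameBP groups nested box actors into a frame that spaces itself from other frames using physics velocity.
; Each tick it pushes all its boxes away from any FrameBP whose center is within range, and nested boxes closer than a threshold push each other apart.
; It also recomputes the boxes' bounds from their locations to place Min and Max markers and update the center used for frame repulsion.
; A sine-driven displacement branch is disconnected.
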(event `self.ReceiveTick`
  (params (DeltaSeconds :type "Float (single-precision)"))
  (bind _minnested (`self.MinNested`))
  (bind _maxnested (`self.MaxNested`))
  (bind _nested (`self.Nested`))
  (bind _returnvalue (`self.K2_GetActorLocation` (`KismetArrayLibrary.Array_Get` (`self.Nested`))))
  ;[1 1 1] Frame Repulsion
  (bind _outactors (`GameplayStatics.GetAllActorsOfClass` "FrameBP_C"))
  (for _array_element _outactors
    (bind _asframe_bp (cast `/Game/FrameBP` _array_element))
    (bind _centernested (`/Game/FrameBP.CenterNested` _asframe_bp))
    (if (and (!= self _array_element) (>= 500.0 (`KismetMathLibrary.VSize` (- _centernested (`self.CenterNested`)))))
      (for _array_element_2 (`self.Nested`)
        (bind _asbox_collision (cast `BoxComponent` (`self.K2_GetRootComponent` _array_element_2)))
        (`PrimitiveComponent.SetPhysicsLinearVelocity` _asbox_collision (* (`KismetMathLibrary.GetForwardVector` (`KismetMathLibrary.FindLookAtRotation` _centernested (`self.CenterNested`))) 3.0) true "None"))))
  ;[1 1 1] Bounds Determination
  (set `self.MaxNested` _returnvalue)
  (set `self.MinNested` _returnvalue)
  (for _array_element_3 (`self.Nested`)
    (bind _x (.x (`self.K2_GetActorLocation` _array_element_3)))
    (bind _y (.y (`self.K2_GetActorLocation` _array_element_3)))
    (bind _z (.z (`self.K2_GetActorLocation` _array_element_3)))
    (set `self.MinNested` (`KismetMathLibrary.MakeVector` (`KismetMathLibrary.FMin` (.x (`self.MinNested`)) _x) (`KismetMathLibrary.FMin` (.y (`self.MinNested`)) _y) (`KismetMathLibrary.FMin` (.z (`self.MinNested`)) _z)))
    (set `self.MaxNested` (`KismetMathLibrary.MakeVector` (`KismetMathLibrary.FMax` _x (.x (`self.MaxNested`))) (`KismetMathLibrary.FMax` _y (.y (`self.MaxNested`))) (`KismetMathLibrary.FMax` _z (.z (`self.MaxNested`))))))
  (`SceneComponent.K2_SetWorldLocation` (`self.Min`) _minnested false false)
  (`SceneComponent.K2_SetWorldLocation` (`self.Max`) _maxnested false false)
  (set `self.CenterNested` (/ (+ _minnested _maxnested) 2.0))
  ;[1 1 1] Box Repulsion
  (for _array_element_4 _nested
    (bind _asbox_actor_bp (cast `/Game/BoxActorBP` _array_element_4))
    (for _array_element_5 _nested
      (bind _asbox_actor_bp_2 (cast `/Game/BoxActorBP` _array_element_5))
      (if (and (>= 200.0 (`self.GetDistanceTo` _asbox_actor_bp _asbox_actor_bp_2)) (!= _asbox_actor_bp _asbox_actor_bp_2))
        (bind _asbox_collision_2 (cast `BoxComponent` (`self.K2_GetRootComponent` _asbox_actor_bp)))
        (`PrimitiveComponent.SetPhysicsLinearVelocity` _asbox_collision_2 (* (`KismetMathLibrary.GetForwardVector` (`KismetMathLibrary.FindLookAtRotation` (`SceneComponent.K2_GetComponentLocation` (`self.K2_GetRootComponent` _asbox_actor_bp_2)) (`SceneComponent.K2_GetComponentLocation` (`self.K2_GetRootComponent` _asbox_actor_bp)))) 9.0) true "None")))))

(fn `UserConstructionScript`)