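; LineActorBP is an actor that links two box actors, From and To, with a beam and pulls them toward each other.
; Construction and Tick update the beam endpoints to From's right socket and To's left socket.
; When the boxes are at least AttractionDistance apart, Tick adds opposing physics velocity to each cube along the line between them.
; Both steps run only when both endpoints are assigned.
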(event `self.ReceiveTick`
  (params (DeltaSeconds :type "Float (single-precision)"))
  (bind _returnvalue (* (`KismetMathLibrary.GetForwardVector` (`KismetMathLibrary.FindLookAtRotation` (`SceneComponent.K2_GetComponentLocation` (`self.K2_GetRootComponent` (`self.From`))) (`SceneComponent.K2_GetComponentLocation` (`self.K2_GetRootComponent` (`self.To`))))) (`self.AttractionVelocity`)))
  (`self.UpdateConnections`)
  ;[1 1 1] Box Attraction
  (bind _newparam (`self.EndpointsAssigned`))
  (if _newparam
    (if (>= (`self.GetDistanceTo` (`self.From`) (`self.To`)) (`self.AttractionDistance`))
      (`PrimitiveComponent.SetPhysicsLinearVelocity` (`BoxActor.cube` (`self.From`)) _returnvalue true "None")
      (`PrimitiveComponent.SetPhysicsLinearVelocity` (`BoxActor.cube` (`self.To`)) (`KismetMathLibrary.NegateVector` _returnvalue) true "None"))))

(fn `EndpointsAssigned`
  (returns (NewParam :type Boolean))
  (return (and (!= (`self.From`) null) (!= (`self.To`) null))))

(fn `UpdateConnections`
  (bind _newparam (`self.EndpointsAssigned`))
  (if _newparam
    (`ParticleSystemComponent.SetBeamSourcePoint` (`self.Beam`) 0 (`SceneComponent.GetSocketLocation` (`/Game/BoxActorBP.StaticMesh` (`self.From`)) "SocketRight") 0)
    (`ParticleSystemComponent.SetBeamTargetPoint` (`self.Beam`) 0 (`SceneComponent.GetSocketLocation` (`/Game/BoxActorBP.StaticMesh` (`self.To`)) "SocketLeft") 0)))

(fn `UserConstructionScript`
  (`self.UpdateConnections`))